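; Archer character Blueprint that fires arrows at a target position and shows an animated target indicator.
; Fire spawns an Arrow at the RightWeaponShield socket and sets its direction from the capsule toward TargetPos.
; TargetEvent extends the parent event, toggling the circle and target components, both hidden at BeginPlay.
; While visible, a looping timer at frame delta interval, used instead of Tick, spins the circle and bobs the target on a sine wave.
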(event Custom|rot%20and%20move
  (bind _target (Variables|Default|GetTarget))
  (bind _cercle (Variables|Default|Getcercle))
  (bind _relativelocation (Variables|/Script/Engine.SceneComponent|GetRelativeLocation _target))
  (bind _relativerotation (Variables|/Script/Engine.SceneComponent|GetRelativeRotation _cercle))
  ;[1 1 1] Rotate Cercle
  (Transformation|SetRelativeRotation _cercle (Math|Rotator|MakeRotator (.roll _relativerotation) (.pitch _relativerotation) (+ (.yaw _relativerotation) (* (Variables|Default|GetspeedRotTarget) (Utilities|Time|GetWorldDeltaSeconds)))) false false)
  ;[1 1 1] Pos Target
  (Transformation|SetRelativeLocation _target (Math|Vector|MakeVector (.x _relativelocation) (.y _relativelocation) (+ (.z _relativelocation) (* (Math|Trig|Sin(Radians) (* (Variables|Default|GetspeedTarget) (Utilities|Time|GetTimeSeconds))) (Variables|Default|GetamplitudeTarget)))) false false))

(event EventFire
  (bind _targetpos (Variables|Default|GettargetPos))
  (bind _capsulecomponent (Variables|Default|GetCapsuleComponent))
  (bind _returnvalue (Transformation|GetWorldLocation _capsulecomponent))
  (bind _returnvalue_2 (- _targetpos _returnvalue))
  (bind _returnvalue_3 (Math|Vector|Normalize _returnvalue_2))
  ;[1 1 1] Shoot
  (bind _returnvalue_4 (Game|SpawnActorfromClass (Variables|NormalAttack|GetArrow) (Math|Transform|MakeTransform (Transformation|GetSocketLocation (Variables|Character|GetMesh) "RightWeaponShield") (Math|Conversions|RotationFromXVector _returnvalue_3)) "AlwaysSpawn" 0 0))
  (if (Utilities|IsValid _returnvalue_4)
    (Variables|/Script/SpookyScuffle.Arrow|Setdirection _returnvalue_4 _returnvalue_3)))

(event EventTargetEvent
  ;[1 1 1] set On/Off visibility
  (|CallParentFunction)
  (Rendering|ToggleVisibility (Variables|Default|Getcercle) false)
  (Rendering|ToggleVisibility (Variables|Default|GetTarget) false)
  (if (Rendering|IsVisible (Variables|Default|GetTarget))
    ;[1 1 1] set timer
    (bind _returnvalue (Utilities|Time|SetTimerbyEvent (delegate Custom|rot%20and%20move) (Utilities|Time|GetWorldDeltaSeconds) true))
    (Variables|Default|SetcontrolTarget _returnvalue)
    (else
      (Utilities|Time|ClearandInvalidateTimerbyHandle (Variables|Default|GetcontrolTarget)))))

(event EventBeginPlay
  ;[1 1 1] Init Variable
  (Rendering|SetVisibility (Variables|Default|Getcercle) false false)
  (Rendering|SetVisibility (Variables|Default|GetTarget) false false))

(fn ConstructionScript)