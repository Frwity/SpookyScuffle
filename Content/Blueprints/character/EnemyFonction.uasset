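; Enemy helper that shows and updates the life bar floating with an enemy.
; BillboardLife shows the Health widget component while the enemy is alive and hides it otherwise.
; It sets the EnemyLifeBar percent to one minus Life over MaxLife, so the bar fills as life drops.
; It billboards by yaw only, turning the widget to face the player's ThirdPersonCharacter follow camera.
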(fn BillboardLife
  (params (IsAlive :type Boolean) (Health :type Widget%20Component%20Object%20Reference) (Life :type Integer) (MaxLife :type Integer))
  ;[1 1 1] Billboard Life
  (bind _asthird_person_character (Utilities|Casting|CastToThirdPersonCharacter (Game|GetPlayerCharacter 0)))
  (if IsAlive
    (Rendering|SetVisibility Health true false)
    (bind _asenemy_life_bar (Utilities|Casting|CastToEnemyLifeBar (UserInterface|GetUserWidgetObject Health)))
    (Progress|SetPercent (Variables|/Game/Blueprints/UI/EnemyLifeBar.EnemyLifeBar_C|GetHealth _asenemy_life_bar) (- 1.0 (/ (Math|Conversions|ToFloat(Integer) Life) (Math|Conversions|ToFloat(Integer) MaxLife))))
    (Transformation|SetWorldRotation Health (Math|Rotator|MakeRotator 0.0 0.0 (+ (.Yaw (Math|Rotator|BreakRotator (Transformation|GetWorldRotation (Variables|/Script/SpookyScuffle.SpookyScuffleCharacter|GetfollowCamera _asthird_person_character)))) 1.8e+02)) false false)
    (else
      (Rendering|SetVisibility Health false false))))