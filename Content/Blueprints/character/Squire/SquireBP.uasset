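; Squire character Blueprint that shows an animated target marker on the Squire and signals when the player is within drain range.
; TargetEvent calls its parent, toggles the Cercle and Target components, and starts or clears a looping, frame-delta timer.
; That timer spins Cercle, bobs Target on a sine wave, and recreates its dynamic material each call, purple in range, original color otherwise.
; An unconnected debug snippet draws the AI controller's strafe target.
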(event Custom|rot%20and%20move
  (bind _target (Variables|Default|GetTarget))
  (bind _cercle (Variables|Default|Getcercle))
  (bind _relativelocation (Variables|/Script/Engine.SceneComponent|GetRelativeLocation _target))
  (bind _relativerotation (Variables|/Script/Engine.SceneComponent|GetRelativeRotation _cercle))
  ;[1 1 1] Rotate Cercle
  (Transformation|SetRelativeRotation _cercle (Math|Rotator|MakeRotator (.roll _relativerotation) (.pitch _relativerotation) (+ (.yaw _relativerotation) (* (Variables|Default|GetspeedRotTarget) (Utilities|Time|GetWorldDeltaSeconds)))) false false)
  ;[1 1 1] Pos Target
  (Transformation|SetRelativeLocation _target (Math|Vector|MakeVector (.x _relativelocation) (.y _relativelocation) (+ (.z _relativelocation) (* (Math|Trig|Sin(Radians) (* (Variables|Default|GetspeedTarget) (Utilities|Time|GetTimeSeconds))) (Variables|Default|GetamplitudeTarget)))) false false)
  ;[1 1 1] Change Color
  (bind _asspooky_scuffle_character (Utilities|Casting|CastToSpookyScuffleCharacter (Game|GetPlayerCharacter 0)))
  (if (< (Math|Vector|VectorLength (- (Transformation|GetActorLocation) (Transformation|GetActorLocation _asspooky_scuffle_character))) (Variables|/Script/SpookyScuffle.SpookyScuffleCharacter|GetdistanceMaxToDrain _asspooky_scuffle_character))
    (bind _returnvalue (Rendering|Material|CreateDynamicMaterialInstance (Variables|Default|GetTarget) 0 "/Game/Platformer/Materials/M_Plastic_Red_Inst.M_Plastic_Red_Inst" "None" :!class /Script/Engine.PrimitiveComponent))
    (Rendering|Material|SetVectorParameterValue _returnvalue "Plastic color" "(R=0.327597,G=0.000000,B=0.427000,A=1.000000)" :!class /Script/Engine.MaterialInstanceDynamic)
    (else
      (bind _returnvalue_2 (Rendering|Material|CreateDynamicMaterialInstance (Variables|Default|GetTarget) 0 "/Game/Platformer/Materials/M_Plastic_Red_Inst.M_Plastic_Red_Inst" "None" :!class /Script/Engine.PrimitiveComponent))
      (Rendering|Material|SetVectorParameterValue _returnvalue_2 "Plastic color" (Variables|Default|GetcolorBase) :!class /Script/Engine.MaterialInstanceDynamic))))

(event EventTargetEvent
  ;[1 1 1] set On/Off visibility
  (|CallParentFunction)
  (Rendering|ToggleVisibility (Variables|Default|Getcercle) false)
  (Rendering|ToggleVisibility (Variables|Default|GetTarget) false)
  (if (Rendering|IsVisible (Variables|Default|GetTarget))
    ;[1 1 1] set timer
    (bind _returnvalue (Utilities|Time|SetTimerbyEvent (delegate Custom|rot%20and%20move) (Utilities|Time|GetWorldDeltaSeconds) true))
    (Variables|Default|SetcontrolTarget _returnvalue)
    (else
      (Utilities|Time|ClearandInvalidateTimerbyHandle (Variables|Default|GetcontrolTarget)))))

(event EventBeginPlay
  ;[1 1 1] Init Variable
  (Rendering|SetVisibility (Variables|Default|Getcercle) false false)
  (Rendering|SetVisibility (Variables|Default|GetTarget) false false)
  (bind _returnvalue (Rendering|Material|CreateDynamicMaterialInstance (Variables|Default|GetTarget) 0 "/Game/Platformer/Materials/M_Plastic_Red_Inst.M_Plastic_Red_Inst" "None" :!class /Script/Engine.PrimitiveComponent))
  (bind _returnvalue_2 (Rendering|Material|GetVectorParameterValue _returnvalue "Plastic color" :!class /Script/Engine.MaterialInstanceDynamic))
  (Variables|Default|SetcolorBase _returnvalue_2))

(fn ConstructionScript)