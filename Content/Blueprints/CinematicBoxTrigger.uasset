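; A one-shot box trigger that plays a level sequence cinematic when overlapped, with a gamepad face-button skip.
; Tick stays disabled until the overlap, then clears all widgets and keeps the SpookyScuffleCharacter immobile while the sequence plays.
; Once it ends or is skipped, Tick restores movement, creates a fresh LifeBar, destroys the trigger and updates the music state through MyGameInstance.
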(event OnComponentBeginOverlap(Box)
  (params (OverlappedComponent :type Primitive%20Component%20Object%20Reference) (OtherActor :type Actor%20Object%20Reference) (OtherComp :type Primitive%20Component%20Object%20Reference) (OtherBodyIndex :type Integer) (bFromSweep :type Boolean) (SweepResult :type Hit%20Result%20Structure%20%28by%20ref%29))
  ;[1 1 1] Launch Cinematic
  (if (Variables|Default|Getcheck)
    (bind _returnvalue (Sequencer|Player|CreateLevelSequencePlayer (Variables|Default|Getcinematic)))
    (bind _output_get (Variables|Default|SetsaveCinematic _returnvalue))
    (Sequencer|Player|Play _output_get :!class /Script/MovieScene.MovieSceneSequencePlayer)
    (Variables|Default|Setcheck false)
    (Variables|Default|SetcinematicOn true)
    (Actor|Tick|SetActorTickEnabled true)))

(event EventTick
  (params (DeltaSeconds :type Float%20%28single-precision%29))
  (if (Variables|Default|GetcinematicOn)
    ;[1 1 1] skip cinematic
    (Viewport|RemoveAllWidgets)
    (if (Game|Player|WasInputKeyJustPressed (Game|GetPlayerController 0) "Gamepad_FaceButton_Bottom")
      (bind _savecinematic (Variables|Default|GetsaveCinematic)
        (:then
          (Class|MovieSceneSequencePlayer|GotoEndandStop _savecinematic)
          (Variables|Default|SetcinematicOn false))
        (:else))
      (else
        ;[1 1 1] player don't move
        (bind _asspooky_scuffle_character (Utilities|Casting|CastToSpookyScuffleCharacter (Game|GetPlayerCharacter 0)))
        (Variables|/Script/SpookyScuffle.SpookyScuffleCharacter|SetplayerMovable _asspooky_scuffle_character false)
        ;[1 1 1] Check End of Cinematic
        (bind _savecinematic_2 (Variables|Default|GetsaveCinematic)
          (:then
            (if (not (Audio|Components|Audio|IsPlaying _savecinematic_2))
              (Variables|Default|SetcinematicOn false)))
          (:else))))
    (else
      ;[1 1 1] End
      (bind _asspooky_scuffle_character_2 (Utilities|Casting|CastToSpookyScuffleCharacter (Game|GetPlayerCharacter 0)))
      (Variables|/Script/SpookyScuffle.SpookyScuffleCharacter|SetplayerMovable _asspooky_scuffle_character_2 true)
      (bind _returnvalue (UserInterface|CreateWidget "/Game/Blueprints/UI/LifeBar.LifeBar_C"))
      (UserInterface|Viewport|AddtoViewport _returnvalue 0)
      (Actor|DestroyActor)
      (bind _asmy_game_instance (Utilities|Casting|CastToMyGameInstance (Game|GetGameInstance)))
      (Default|UpdateMusic _asmy_game_instance "NewEnumerator2" false))))

(event EventBeginPlay
  ;[1 1 1] disable tick
  (Actor|Tick|SetActorTickEnabled false))

(fn ConstructionScript)