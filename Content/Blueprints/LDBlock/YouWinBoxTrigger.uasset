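; YouWinBoxTrigger is a trigger actor that handles the win and ending when a player character reaches it.
; Any actor overlap by a ThirdPersonCharacter calls that character's YouWinEvent.
; Separately, a SpookyScuffleCharacter entering the Box is hidden on every overlap.
; A Check flag gates a one-time playback of the CinematicEnd level sequence, followed by a music state change through MyGameInstance.
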(event OnComponentBeginOverlap(Box)
  (params (OverlappedComponent :type Primitive%20Component%20Object%20Reference) (OtherActor :type Actor%20Object%20Reference) (OtherComp :type Primitive%20Component%20Object%20Reference) (OtherBodyIndex :type Integer) (bFromSweep :type Boolean) (SweepResult :type Hit%20Result%20Structure%20%28by%20ref%29))
  (bind _asspooky_scuffle_character (Utilities|Casting|CastToSpookyScuffleCharacter OtherActor))
  (Rendering|SetActorHiddenInGame _asspooky_scuffle_character true)
  (if (Variables|Default|GetCheck)
    (Variables|Default|SetCheck false)
    (bind _returnvalue (Sequencer|Player|CreateLevelSequencePlayer (Variables|Default|GetCinematicEnd)))
    (Sequencer|Player|Play _returnvalue :!class /Script/MovieScene.MovieSceneSequencePlayer)
    (bind _asmy_game_instance (Utilities|Casting|CastToMyGameInstance (Game|GetGameInstance)))
    (Default|UpdateMusic _asmy_game_instance "NewEnumerator6" false)))

(event Collision|EventActorBeginOverlap
  (params (OtherActor :type Actor%20Object%20Reference))
  ;[1 1 1] Call You Win Event
  (bind _asthird_person_character (Utilities|Casting|CastToThirdPersonCharacter OtherActor))
  (Class|SpookyScuffleCharacter|YouWinEvent _asthird_person_character))

(fn ConstructionScript)