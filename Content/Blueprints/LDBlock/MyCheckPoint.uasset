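; MyCheckPoint is a level-design checkpoint actor that gives one-time visual and audio feedback when its Box is first overlapped.
; The overlap, with no check on the overlapping actor, activates Smoke, plays an optional 2D sound and clears the FirstCheck flag.
; It also starts a looping timer at the current frame's delta time, standing in for Tick, which rolls Scene until it passes RotateValue.
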(event OnComponentBeginOverlap(Box)
  (params (OverlappedComponent :type Primitive%20Component%20Object%20Reference) (OtherActor :type Actor%20Object%20Reference) (OtherComp :type Primitive%20Component%20Object%20Reference) (OtherBodyIndex :type Integer) (bFromSweep :type Boolean) (SweepResult :type Hit%20Result%20Structure%20%28by%20ref%29))
  (if (Variables|Default|GetfirstCheck)
    (bind _returnvalue (Utilities|Time|SetTimerbyEvent (delegate Custom|Rotate) (Utilities|Time|GetWorldDeltaSeconds) true))
    (Variables|Default|SetcheckRotate _returnvalue)
    (Components|Activation|Activate (Variables|Default|Getsmoke) true)
    (Variables|Default|SetfirstCheck false)
    (bind _soundcheckpoint (Variables|Default|GetsoundCheckPoint)
      (:then
        (Audio|PlaySound2D _soundcheckpoint 1.0 1.0 0.0 0 0))
      (:else))))

(event Custom|Rotate
  (bind _scene (Variables|Default|GetScene))
  (bind _returnvalue (Transformation|GetWorldRotation _scene))
  ;[1 1 1] Rotate
  (if (<= (.roll _returnvalue) (Variables|Default|GetrotateValue))
    (Transformation|SetWorldRotation (Variables|Default|GetScene) (Math|Rotator|MakeRotator (+ (.roll _returnvalue) (* (Variables|Default|GetspeedRotate) (Utilities|Time|GetWorldDeltaSeconds))) (.pitch _returnvalue) (.yaw _returnvalue)) false false)
    (else
      (Utilities|Time|ClearandInvalidateTimerbyHandle (Variables|Default|GetcheckRotate)))))

(fn ConstructionScript)