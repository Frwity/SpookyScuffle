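; Game instance that keeps player camera options and controls state-based music for the game.
; Init runs once, caching axis inversion and sensitivity from SpookyScuffleCharacter and applying master volume through a sound mix class override.
; SetOption writes cached options back, but casts to ThirdPersonCharacter instead.
; UpdateMusic stops the current track and spawns the new state's 2D cue, skipping unchanged states unless forced.
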(fn SaveOption
  (bind _asspooky_scuffle_character (Utilities|Casting|CastToSpookyScuffleCharacter (Game|GetPlayerCharacter 0)))
  (Variables|Default|SetInvertX (Variables|/Script/SpookyScuffle.SpookyScuffleCharacter|GetinvertXAxis _asspooky_scuffle_character))
  (Variables|Default|SetInvertZ (Variables|/Script/SpookyScuffle.SpookyScuffleCharacter|GetinvertZAxis _asspooky_scuffle_character))
  (Variables|Default|SetSensiX (Variables|/Script/SpookyScuffle.SpookyScuffleCharacter|GetsensibilityX _asspooky_scuffle_character))
  (Variables|Default|SetSensiZ (Variables|/Script/SpookyScuffle.SpookyScuffleCharacter|GetsensibilityZ _asspooky_scuffle_character)))

(fn SetOption
  (bind _asthird_person_character (Utilities|Casting|CastToThirdPersonCharacter (Game|GetPlayerCharacter 0)))
  (Variables|/Script/SpookyScuffle.SpookyScuffleCharacter|SetinvertZAxis _asthird_person_character (Variables|Default|GetInvertZ))
  (Variables|/Script/SpookyScuffle.SpookyScuffleCharacter|SetinvertXAxis _asthird_person_character (Variables|Default|GetInvertX))
  (Variables|/Script/SpookyScuffle.SpookyScuffleCharacter|SetsensibilityX _asthird_person_character (Variables|Default|GetSensiX))
  (Variables|/Script/SpookyScuffle.SpookyScuffleCharacter|SetsensibilityZ _asthird_person_character (Variables|Default|GetSensiZ)))

(fn Init
  (if (not (Variables|Default|GetIsInit))
    (CallFunction|SaveOption)
    (Variables|Default|SetIsInit true)
    (Audio|SetSoundMixClassOverride "/Game/Sounds/GlobalSoundMix.GlobalSoundMix" "/Game/Sounds/GlobalSoundClass.GlobalSoundClass" (/ (Variables|Default|GetVolume) 1e+01) 1.0 1.0 true)))

(fn UpdateMusic
  (params (NewMusicState :type E_MUSIC%20Enum :default "NewEnumerator0") (Force :type Boolean))
  (if (or Force (not (== NewMusicState (Variables|Default|GetMusic))))
    (Variables|Default|SetMusic NewMusicState)
    (if (Utilities|IsValid (Variables|Sound|GetCurrentMusic))
      (Audio|Components|Audio|Stop (Variables|Sound|GetCurrentMusic)))
    (switch Utilities|FlowControl|Switch|SwitchonE_MUSIC (Variables|Default|GetMusic)
      (:NewEnumerator0
        (bind _returnvalue (Audio|SpawnSound2D "/Game/Sounds/S_Menu_Music_Cue.S_Menu_Music_Cue" 1.0 1.0 0.0 0))
        (Variables|Sound|SetCurrentMusic _returnvalue))
      (:NewEnumerator1
        (bind _returnvalue_2 (Audio|SpawnSound2D "/Game/Sounds/S_Menu_LobbyScreen_Music_Cue.S_Menu_LobbyScreen_Music_Cue" 1.0 1.0 0.0 0 true))
        (Variables|Sound|SetCurrentMusic _returnvalue_2))
      (:NewEnumerator4
        (bind _returnvalue_3 (Audio|SpawnSound2D "/Game/Sounds/S_System_Tutorial_Music_Cue.S_System_Tutorial_Music_Cue" 1.0 1.0 0.0 0 true false))
        (Variables|Sound|SetCurrentMusic _returnvalue_3))
      (:NewEnumerator2
        (bind _returnvalue_4 (Audio|SpawnSound2D "/Game/Sounds/S_System_Ingame_Music_Cue.S_System_Ingame_Music_Cue" 0.5 1.0 0.0 0 true))
        (Variables|Sound|SetCurrentMusic _returnvalue_4))
      (:NewEnumerator5
        (bind _returnvalue_5 (Audio|SpawnSound2D "/Game/Sounds/S_System_ThirdArenaMusic_Cue.S_System_ThirdArenaMusic_Cue" 0.5 1.0 0.0 0 true))
        (Variables|Sound|SetCurrentMusic _returnvalue_5))
      (:NewEnumerator6
        (bind _returnvalue_6 (Audio|SpawnSound2D "/Game/Sounds/S_System_Victory_Jingle_Cue.S_System_Victory_Jingle_Cue" 1.0 1.0 0.0 0))
        (Variables|Sound|SetCurrentMusic _returnvalue_6)))))