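; Archer Blueprint whose Fire event shoots an Arrow toward TargetPos.
; The arrow always spawns, regardless of collision, at the mesh's RightWeaponShield socket.
; Its rotation and Direction both come from the normalized vector from the capsule's location to TargetPos, so aim is measured from the capsule rather than the socket.
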(event EventFire
  (bind _targetpos (Variables|Default|GettargetPos))
  (bind _capsulecomponent (Variables|Default|GetCapsuleComponent))
  (bind _returnvalue (Transformation|GetWorldLocation _capsulecomponent))
  (bind _returnvalue_2 (- _targetpos _returnvalue))
  (bind _returnvalue_3 (Math|Vector|Normalize _returnvalue_2))
  (bind _returnvalue_4 (Game|SpawnActorfromClass (Variables|NormalAttack|GetArrow) (Math|Transform|MakeTransform (Transformation|GetSocketLocation (Variables|Character|GetMesh) "RightWeaponShield") (Math|Conversions|RotationFromXVector _returnvalue_3)) "AlwaysSpawn" 0 0))
  (if (Utilities|IsValid _returnvalue_4)
    (Variables|/Script/SpookyScuffle.Arrow|Setdirection _returnvalue_4 _returnvalue_3)))

(fn ConstructionScript)