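; MyHUD is the HUD Blueprint that creates the menu screens for Spooky Scuffle.
; On BeginPlay it disables movement on the player's SpookyScuffleCharacter and opens the MainMenu widget.
; ShowPauseMenu toggles a single Pause widget, cached in SaveWidget while it is shown.
; ShowEndMenu adds the GameOver screen, while ShowWinMenu clears all widgets before adding the Win screen.
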(event EventBeginPlay
  ;[1 1 1] Main Menu
  (bind _asspooky_scuffle_character (Utilities|Casting|CastToSpookyScuffleCharacter (Game|GetPlayerCharacter 0)))
  (Variables|/Script/SpookyScuffle.SpookyScuffleCharacter|SetplayerMovable _asspooky_scuffle_character false)
  (bind _returnvalue (UserInterface|CreateWidget "/Game/Blueprints/MainMenu.MainMenu_C" (Game|GetPlayerController 0)))
  (UserInterface|Viewport|AddtoViewport _returnvalue 0))

(fn ConstructionScript)

(fn ShowPauseMenu
  (params (isPause :type Boolean))
  (if isPause
    ;[1 1 1] Create Widget Pause
    (Variables|Default|GetsaveWidget
      (:then)
      (:else
        (bind _returnvalue (UserInterface|CreateWidget "/Game/Blueprints/Pause.Pause_C" (Game|GetPlayerController 0)))
        (bind _output_get (Variables|Default|SetsaveWidget _returnvalue))
        (UserInterface|Viewport|AddtoViewport _output_get 0)))
    (else
      ;[1 1 1] Destroy Widget
      (bind _savewidget (Variables|Default|GetsaveWidget)
        (:then
          (Widget|RemovefromParent _savewidget)
          (Variables|Default|SetsaveWidget 0))
        (:else)))))

(fn ShowEndMenu
  ;[1 1 1] Create GameOver Screen
  (bind _returnvalue (UserInterface|CreateWidget "/Game/Blueprints/GameOver.GameOver_C" (Game|GetPlayerController 0)))
  (UserInterface|Viewport|AddtoViewport _returnvalue 0)
  (return))

(fn ShowWinMenu
  ;[1 1 1] Show Win Screen
  (Viewport|RemoveAllWidgets)
  (bind _returnvalue (UserInterface|CreateWidget "/Game/Blueprints/Win.Win_C" (Game|GetPlayerController 0)))
  (UserInterface|Viewport|AddtoViewport _returnvalue 0)
  (return))